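; Dragon enemy character that roars, chases the player and plays a claw attack montage on reaching them.
; Tick and pawn sensing share one chase path, so pursuit runs regardless of sight, gated by alive, movement and hit-reaction flags.
; Trigger events start and stop a looping timer that line-traces between mesh sockets to damage the player.
; Damage plays hit or death montages; death destroys the dragon, fires OnDestroyed and awards money and score.
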(event `CustomEvent`
  (params (`On/Off` :type Boolean))
  (bind _output_get (set `self.CanMove` `On/Off`))
  (set `self.canAttack` _output_get))

(event `self.ReceiveAnyDamage`
  (params (Damage :type "Float (single-precision)") (DamageType :type "DamageType Object Reference") (InstigatedBy :type "Controller Object Reference") (DamageCauser :type "Actor Object Reference"))
  (bind _charactermovement (`self.CharacterMovement`))
  ;[1 1 1] Comment
  (set `self.IsAnimate` true)
  (`/Engine/EditorBlueprintResources/StandardMacros.DoOnce` false :!label _label
    (:`Completed`
      (bind _output_get (set `self.Health` (- (`self.Health`) Damage)))
      (if (<= _output_get 0.0)
        (set `self.isSeeingPlayer` false)
        (set `self.IsAlive` false)
        (bind _returnvalue (`self.PlayAnimMontage` "/Game/QuadrapedCreatures/MountainDragon/Animations/ANIM_MOUNTAIN_DRAGON_death_Montage.ANIM_MOUNTAIN_DRAGON_death_Montage" 0.9))
        (`GameplayStatics.PlaySoundAtLocation` "/Game/Sounds/Dragon/Dragon_dead.Dragon_dead" (`self.K2_GetActorLocation`) (struct) 1.0 1.0 0.0 null null null)
        (`CharacterMovementComponent.DisableMovement` (`self.CharacterMovement`))
        (`KismetSystemLibrary.Delay` _returnvalue)
        (`self.K2_DestroyActor`)
        (`self.On Destroyed`)
        (bind _asthird_person_character (cast `/Game/ThirdPersonBP/Blueprints/ThirdPersonCharacter` (`GameplayStatics.GetPlayerCharacter` 0)))
        (set `/Game/ThirdPersonBP/Blueprints/ThirdPersonCharacter.Money` (+ (`/Game/ThirdPersonBP/Blueprints/ThirdPersonCharacter.Money` _asthird_person_character) 20) _asthird_person_character)
        (set `/Game/ThirdPersonBP/Blueprints/ThirdPersonCharacter.Score` (+ (`/Game/ThirdPersonBP/Blueprints/ThirdPersonCharacter.Score` _asthird_person_character) 300) _asthird_person_character)
        (else
          (bind _returnvalue_2 (`self.PlayAnimMontage` "/Game/QuadrapedCreatures/MountainDragon/Animations/ANIM_MOUNTAIN_DRAGON_getHitLeft_Montage.ANIM_MOUNTAIN_DRAGON_getHitLeft_Montage"))
          (`CharacterMovementComponent.DisableMovement` _charactermovement)
          (`KismetSystemLibrary.Delay` _returnvalue_2)
          (set `self.IsAnimate` false)
          (`CharacterMovementComponent.SetMovementMode` _charactermovement "MOVE_Walking" 0)
          (goto _label :!via `Reset`))))))

(event `self.ReceiveTick`
  (params (DeltaSeconds :type "Float (single-precision)"))
  ;[1 1 1] Move To Player
  (set `self.isSeeingPlayer` true :!label _label_2)
  (`self.DFollowPlayer`)
  (if (`self.IsAlive`)
    (`|ExecutionSequence`
      (:`then_0`
        (`/Engine/EditorBlueprintResources/StandardMacros.DoOnce` false :!label _label_3
          (:`Completed`
            (bind _returnvalue (`GameplayStatics.SpawnSoundAtLocation` "/Game/Sounds/Dragon/Dragon_roar_sound_effect_.Dragon_roar_sound_effect_" (`self.K2_GetActorLocation`) (struct) 1.0 1.0 0.0 null null false)))))
      (:`then_1`
        (`KismetSystemLibrary.RetriggerableDelay` 1.0)
        (goto _label_3 :!via `Reset`)))
    (else
      (`AudioComponent.Stop` _returnvalue))))

(event `self.PawnSensing.OnSeePawn`
  (params (Pawn :type "Pawn Object Reference"))
  ;[1 1 1] Move To Player
  (goto _label_2))

(event `DFollowPlayer`
  (bind _charactermovement (`self.CharacterMovement`))
  ;[1 1 1] Move To Player
  (set `self.canAttack` true)
  (if (and (`self.isSeeingPlayer`) (`self.IsAlive`) (not (`self.IsAnimate`)))
    (if (`self.CanMove`)
      (`|AIMoveTo` self (0.0 0.0 0.0) (`GameplayStatics.GetPlayerCharacter` 0) 300.0
        (:`OnSuccess`
          (if (`self.canAttack`)
            (set `self.canAttack` false)
            (`/Engine/EditorBlueprintResources/StandardMacros.DoOnce` false :!label _label_4
              (:`Completed`
                (bind _returnvalue (`self.PlayAnimMontage` "/Game/QuadrapedCreatures/MountainDragon/Animations/ANIM_MOUNTAIN_DRAGON_rightClawsAttackForward_Montage.ANIM_MOUNTAIN_DRAGON_rightClawsAttackForward_Montage"))
                (`CharacterMovementComponent.DisableMovement` _charactermovement)
                (`KismetSystemLibrary.Delay` _returnvalue)
                (`CharacterMovementComponent.SetMovementMode` _charactermovement "MOVE_Walking" 0)
                (set `self.canAttack` true)
                (goto _label_4 :!via `Reset`)))))))))

(event `Trigger Dhand`
  ;[1 1 1] Comment
  (bind _returnvalue (`KismetSystemLibrary.K2_SetTimerDelegate` (delegate `DHandLineTrace`) 0.01 true))
  (set `self.HandTrigger` _returnvalue))

(event `DHandLineTrace`
  (bind _mesh (`self.Mesh`))
  ;[1 1 1] Comment
  (bind _outhit (`KismetSystemLibrary.LineTraceSingle` (`SceneComponent.GetSocketLocation` _mesh "Start") (`SceneComponent.GetSocketLocation` _mesh "End") "TraceTypeQuery2"))
  (bind (_bblockinghit _binitialoverlap _time _distance _location _impactpoint _normal _impactnormal _physmat _hitactor) (`GameplayStatics.BreakHitResult` _outhit))
  (if (== _hitactor (`GameplayStatics.GetPlayerCharacter` 0))
    (`GameplayStatics.ApplyDamage` _hitactor 20.0)))

(event `StopTriggerDhand`
  ;[1 1 1] Comment
  (`KismetSystemLibrary.K2_ClearAndInvalidateTimerHandle` (`self.HandTrigger`)))

(fn `FollowPlayer`)

(fn `UserConstructionScript`)