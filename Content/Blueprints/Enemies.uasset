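; Enemy character Blueprint that stands still until it sees a pawn, then chases the player and attacks.
; PawnSensing sets a seen flag, which in practice stays set, and starts an AI MoveTo toward the player character.
; On arrival it calls PlayAnimMontage, gated by a CanAttack flag and a delay for the montage length.
; Random wandering and destroy-on-overlap logic exist but are disconnected.
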(event `self.ReceiveBeginPlay`)

(event `Move`
  ;[1 1 1] AI Stupid Move
  (`|AIMoveTo` self (`NavigationSystemV1.K2_GetRandomReachablePointInRadius` (`self.K2_GetActorLocation`) 300.0 null null) null
    (:`OnSuccess`
      (`KismetSystemLibrary.Delay` 3.0)
      (`self.Move`))))

(event `self.Box.OnComponentBeginOverlap`
  (params (OverlappedComponent :type "PrimitiveComponent Object Reference") (OtherActor :type "Actor Object Reference") (OtherComp :type "PrimitiveComponent Object Reference") (OtherBodyIndex :type Integer) (bFromSweep :type Boolean) (SweepResult :type "HitResult Structure (by ref)")))

(event `self.ReceiveTick`
  (params (DeltaSeconds :type "Float (single-precision)"))
  (if (not (`self.isSeeingPlayer`))
    (`MovementComponent.StopMovementImmediately` (`self.CharacterMovement`))))

(event `self.PawnSensing.OnSeePawn`
  (params (Pawn :type "Pawn Object Reference"))
  (set `self.isSeeingPlayer` true)
  (`self.FollowPlayer`))

(event `FollowPlayer`
  (set `self.canAttack` true)
  (if (`self.isSeeingPlayer`)
    (`|AIMoveTo` self (0.0 0.0 0.0) (`GameplayStatics.GetPlayerCharacter` 0) 70.0
      (:`OnSuccess`
        (if (`self.canAttack`)
          (set `self.canAttack` false)
          (bind _returnvalue (`self.PlayAnimMontage` null))
          (`KismetSystemLibrary.Delay` _returnvalue)
          (set `self.canAttack` true))))
    (else
      (set `self.isSeeingPlayer` false))))

(fn `UserConstructionScript`)