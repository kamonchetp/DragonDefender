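; BP_EnemyPortal is an enemy spawner that creates BP_TheEnemy AI pawns at the location of its PortalBox component.
; It exposes Easy, Medium and Hard events, which all run identical logic with no difference between difficulties.
; Each call counts every BP_TheEnemy in the world and spawns one more only while that count is under a shared hard-coded cap of 100.
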(event `Easy`
  (bind _outactors (`GameplayStatics.GetAllActorsOfClass` "/Game/Blueprints/Enemy/BP_TheEnemy.BP_TheEnemy_C"))
  (if (< (`KismetArrayLibrary.Array_Length` _outactors) 100)
    (`AIBlueprintHelperLibrary.SpawnAIFromClass` "/Game/Blueprints/Enemy/BP_TheEnemy.BP_TheEnemy_C" null (`SceneComponent.K2_GetComponentLocation` (`self.PortalBox`)) (struct) false null)))

(event `Medium`
  (bind _outactors (`GameplayStatics.GetAllActorsOfClass` "/Game/Blueprints/Enemy/BP_TheEnemy.BP_TheEnemy_C"))
  (if (< (`KismetArrayLibrary.Array_Length` _outactors) 100)
    (`AIBlueprintHelperLibrary.SpawnAIFromClass` "/Game/Blueprints/Enemy/BP_TheEnemy.BP_TheEnemy_C" null (`SceneComponent.K2_GetComponentLocation` (`self.PortalBox`)) (struct) false null)))

(event `Hard`
  (bind _outactors (`GameplayStatics.GetAllActorsOfClass` "/Game/Blueprints/Enemy/BP_TheEnemy.BP_TheEnemy_C"))
  (if (< (`KismetArrayLibrary.Array_Length` _outactors) 100)
    (`AIBlueprintHelperLibrary.SpawnAIFromClass` "/Game/Blueprints/Enemy/BP_TheEnemy.BP_TheEnemy_C" null (`SceneComponent.K2_GetComponentLocation` (`self.PortalBox`)) (struct) false null)))

(fn `UserConstructionScript`)