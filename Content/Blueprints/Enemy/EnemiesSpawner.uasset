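; Enemy spawner actor that works through a queue of enemy classes, spawning each at its own transform.
; AddEnemyToQ appends a class and spawns the front entry immediately if no enemies overlap the Sphere.
; A looping timer also spawns from the queue, without that overlap check.
; Spawned enemies get a destroyed-event binding, and OnEnemyDefeated forwards defeats to ThirdPersonGameMode.
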(event `self.ReceiveBeginPlay`
  (`KismetSystemLibrary.K2_SetTimerDelegate` (delegate `TryToSpawn`) 2.0 true))

(event `TryToSpawn`
  (`self.SpawnEnemy`))

(event `OnEnemyDefeated`
  (bind _asthird_person_game_mode (cast `/Game/ThirdPersonBP/Blueprints/ThirdPersonGameMode` (`GameplayStatics.GetGameMode`)))
  (`/Game/ThirdPersonBP/Blueprints/ThirdPersonGameMode.OnEnemyDefeated` _asthird_person_game_mode))

(fn `AddEnemyToQ`
  (params (EnemyClass :type "/Game/Blueprints/Enemy/Enemies Class Reference (by ref)"))
  (`KismetArrayLibrary.Array_Add` (`self.EnemyQ`) EnemyClass)
  (if (not (`KismetArrayLibrary.Array_IsValidIndex` (`PrimitiveComponent.GetOverlappingActors` (`self.Sphere`) "/Game/Blueprints/Enemy/Enemies.Enemies_C")))
    (`self.SpawnEnemy`)))

(fn `SpawnEnemy`
  (returns (Success :type Boolean))
  (if (`KismetArrayLibrary.Array_IsValidIndex` (`self.EnemyQ`))
    (bind _returnvalue (`|SpawnActorFromClass` (`|GetArrayItem` (`self.EnemyQ`)) (`self.GetTransform`) "AdjustIfPossibleButAlwaysSpawn" "OverrideRootScale" null null))
    (add `/Game/Blueprints/Enemy/Enemies.On Destroyed` _returnvalue (`|CreateDelegate` :!event `OnEnemyDefeated`))
    (`KismetArrayLibrary.Array_Remove` (`self.EnemyQ`))
    (return true)
    (else
      (return false))))

(fn `UserConstructionScript`)